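; Actor component for MoSysCameraNDisplay that syncs lens focus across an nDisplay cluster.
; It registers as a cluster event listener for the duration of play.
; On non-master nodes, "lensData" JSON events set the owning camera's CineCamera manual focus distance from the "focus" parameter.
; The camera's focus method must be set to manual.
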(event EventBeginPlay
  (Class|DisplayClusterBlueprintAPI|AddClusterEventListener (Class|DisplayClusterBlueprintLib|GetAPI) self))

(event EventOnClusterEventJson
  (params (Event :type Display%20Cluster%20Cluster%20Event%20Json%20Structure%20%28by%20ref%29))
  (bind (_name _type _category _parameters) (Utilities|Struct|BreakDisplayClusterClusterEventJson Event))
  ;[1 1 1] Listen to focus event from lens control. Set focus to manual on MoSysCameraNDisplay!
  (if (not (Class|DisplayClusterBlueprintAPI|IsMaster (Class|DisplayClusterBlueprintLib|GetAPI)))
    (if (Utilities|Enum|Equal(Enum) _name "lensData")
      (bind _asmo_sys_camera_ndisplay (Utilities|Casting|CastToMoSysCameraNDisplay (Components|GetOwner)))
      (Utilities|Struct|SetmembersinCameraFocusSettings (Variables|/Script/CinematicCamera.CineCameraComponent|GetFocusSettings (Class|CineCameraActor|GetCineCameraComponent _asmo_sys_camera_ndisplay)) (Math|Conversions|ToFloat(Integer) (.Value (Utilities|Map|Find _parameters "focus")))))))

(event EventEndPlay
  (params (EndPlayReason :type EEndPlayReason%20Enum :default "Destroyed"))
  (Class|DisplayClusterBlueprintAPI|RemoveClusterEventListener (Class|DisplayClusterBlueprintLib|GetAPI) self))